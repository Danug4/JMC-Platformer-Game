(event OnComponentBeginOverlap(Collision)
  (params (OverlappedComponent :type Primitive%20Component%20Object%20Reference) (OtherActor :type Actor%20Object%20Reference) (OtherComp :type Primitive%20Component%20Object%20Reference) (OtherBodyIndex :type Integer) (bFromSweep :type Boolean) (SweepResult :type Hit%20Result%20Structure%20%28by%20ref%29))
  (bind _player (Variables|Default|GetPlayer))
  (bind _player_2 (Variables|Default|GetPlayer))
  ;[0.0575 0.06226 0.15 0.5] Player brings NPC to its home
  (if (== OtherActor _player)
    (if (Variables|/Game/ThirdPerson/Blueprints/BP_ThirdPersonCharacter.BP_ThirdPersonCharacter_C|GetIsHoldingNPC _player)
      (Variables|/Game/ThirdPerson/Blueprints/BP_ThirdPersonCharacter.BP_ThirdPersonCharacter_C|SetIsHoldingNPC _player false)
      (Utilities|FlowControl|Sequence
        (:then_0
          ;;[0.05276 0.06895 0.15 0.5] Hide NPC on player
          (Default|HideNPCHolder _player_2))
        (:then_1
          ;;[0.04806 0.06881 0.15 0.5] Reward Player
          (Default|RewardPlayer _player_2))
        (:then_2
          ;;[0.0556 0.06801 0.15 0.5] Spawn Thankyou NPC
          (Game|SpawnActorfromClass "/Game/Platformer/Blueprints/BP_NPC_Lost_Completed.BP_NPC_Lost_Completed_C" (Math|Transform|MakeTransform (Transformation|GetWorldLocation (Variables|Default|GetNPCSpawnPoint)) "0, 0, 0" "1.000000,1.000000,1.000000") "Undefined" "MultiplyWithRoot" 0 0))))))

(event EventBeginPlay
  ;[0.03449 0.04915 0.15 0.5] Reference Player
  (bind _asbp_third_person_character (Utilities|Casting|CastToBP_ThirdPersonCharacter (Game|Player|GetPlayerPawn 0)))
  (Variables|Default|SetPlayer _asbp_third_person_character))

(fn ConstructionScript)
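; Platformer platform that vanishes after the player pawn stands on it too long, then reappears.
; Trigger zone overlaps set a flag that lets Tick accumulate time on the platform, resetting it when the player is off.
; At the lifetime limit it hides and disables collision, then after a delay restores both and sets the trigger zone to the saved start transform.
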(event OnComponentBeginOverlap(PlatformTriggerZone)
  (params (OverlappedComponent :type Primitive%20Component%20Object%20Reference) (OtherActor :type Actor%20Object%20Reference) (OtherComp :type Primitive%20Component%20Object%20Reference) (OtherBodyIndex :type Integer) (bFromSweep :type Boolean) (SweepResult :type Hit%20Result%20Structure%20%28by%20ref%29))
  (if (== OtherActor (Game|Player|GetPlayerPawn 0))
    (Utilities|FlowControl|Sequence
      (:then_0
        (Development|PrintString "Player on platform"))
      (:then_1
        (Variables|Default|SetIsPlayerOnPlatform true)))))

(event OnComponentEndOverlap(PlatformTriggerZone)
  (params (OverlappedComponent :type Primitive%20Component%20Object%20Reference) (OtherActor :type Actor%20Object%20Reference) (OtherComp :type Primitive%20Component%20Object%20Reference) (OtherBodyIndex :type Integer))
  (if (== OtherActor (Game|Player|GetPlayerPawn 0))
    (Utilities|FlowControl|Sequence
      (:then_0
        (Development|PrintString "Player off platform"))
      (:then_1
        (Variables|Default|SetIsPlayerOnPlatform false)))))

(event Custom|Toggle-Object
  (params (IsHidden :type Boolean) (CollisionEnabled :type Boolean))
  ;[0.02173 0.15 0.07758 0.5] Turn Visibility and Collision On / Off
  (Rendering|SetActorHiddenInGame IsHidden)
  (Collision|SetActorEnableCollision CollisionEnabled))

(event Custom|ReturnToStart
  (Transformation|SetWorldTransform (Variables|Default|GetPlatformTriggerZone) (Variables|Default|GetStartTransform) false false)
  (Variables|Default|SetTimeOnPlatform 0.0)
  (CallFunction|Toggle-Object false true))

(event EventBeginPlay
  (Variables|Default|SetStartTransform (Transformation|GetActorTransform))
  ;[0.15 0.15 0.15 0.5] Setup current time on platform to max
  (Variables|Default|SetTimeOnPlatform (Variables|Default|GetPlatformLifetime)))

(event EventTick
  (params (DeltaSeconds :type Float%20%28single-precision%29))
  ;[0.15 0.15 0.15 0.5] Set Timer for platform
  (if (Variables|Default|GetIsPlayerOnPlatform)
    (bind _output_get (Variables|Default|SetTimeOnPlatform (+ DeltaSeconds (Variables|Default|GetTimeOnPlatform))))
    (Development|PrintString (Utilities|String|ToString(Float) _output_get))
    ;[0.15 0.15 0.15 0.5] Check timer life
    (if (>= (Variables|Default|GetTimeOnPlatform) (Variables|Default|GetPlatformLifetime))
      ;[0.15 0.15 0.15 0.5] Hide & disable platform
      (CallFunction|Toggle-Object true false)
      (Utilities|FlowControl|Delay (Variables|Default|GetTimeInvisible))
      (CallFunction|ReturntoStart))
    (else
      (Variables|Default|SetTimeOnPlatform 0.0))))

(fn ConstructionScript)
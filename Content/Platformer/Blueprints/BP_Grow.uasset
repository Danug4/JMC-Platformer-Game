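; BP_Grow is a platformer actor, a tree that grows when the player enters its trigger.
; BeginPlay records the ScaleParent component's Z scale as the end scale, then sets it uniformly to StartScale.
; When the player pawn overlaps Collision, the TreeGrow timeline plays, lerping ScaleParent uniformly from start to end scale.
; Each timeline update also prints a "Growing" message.
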(event OnComponentBeginOverlap(Collision)
  (params (OverlappedComponent :type Primitive%20Component%20Object%20Reference) (OtherActor :type Actor%20Object%20Reference) (OtherComp :type Primitive%20Component%20Object%20Reference) (OtherBodyIndex :type Integer) (bFromSweep :type Boolean) (SweepResult :type Hit%20Result%20Structure%20%28by%20ref%29))
  ;[0.15 0.15 0.15 0.5] If Player enters trigger zone: grow the tree
  (if (== OtherActor (Game|Player|GetPlayerPawn 0))
    (bind _grow (Timeline|Tree-Grow Play)
      (:Update
        (Development|PrintString "Growing")
        (Transformation|SetRelativeScale3D (Variables|Default|GetScaleParent) (Math|Vector|MakeVector (Math|Float|Lerp (Variables|Default|GetStartScale) (Variables|Default|GetEndScale) _grow) (Math|Float|Lerp (Variables|Default|GetStartScale) (Variables|Default|GetEndScale) _grow) (Math|Float|Lerp (Variables|Default|GetStartScale) (Variables|Default|GetEndScale) _grow)))))))

(event EventBeginPlay
  (bind _startscale (Variables|Default|GetStartScale))
  ;[0.15 0.15 0.15 0.5] Set end scale to current scale, and set the current scale to start scale
  (Variables|Default|SetEndScale (.z (Variables|/Script/Engine.SceneComponent|GetRelativeScale3D (Variables|Default|GetScaleParent))))
  (Transformation|SetRelativeScale3D (Variables|Default|GetScaleParent) (Math|Vector|MakeVector _startscale _startscale _startscale)))

(fn ConstructionScript)
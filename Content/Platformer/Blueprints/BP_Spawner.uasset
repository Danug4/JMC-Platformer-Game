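; BP_Spawner is a pickup actor that grants the player the spawner item.
; On BeginPlay it caches the player pawn as a BP_ThirdPersonCharacter reference.
; When that player overlaps its Trigger component, it sets the character's HoldSpawner flag, plays the Coinrecieved sound at the player's location, and destroys itself.
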(event OnComponentBeginOverlap(Trigger)
  (params (OverlappedComponent :type Primitive%20Component%20Object%20Reference) (OtherActor :type Actor%20Object%20Reference) (OtherComp :type Primitive%20Component%20Object%20Reference) (OtherBodyIndex :type Integer) (bFromSweep :type Boolean) (SweepResult :type Hit%20Result%20Structure%20%28by%20ref%29))
  (bind _player (Variables|Default|GetPlayer))
  ;[0.15 0.01297 0.1478 0.5] Pickup Spawner
  (if (== OtherActor _player)
    (Variables|/Game/ThirdPerson/Blueprints/BP_ThirdPersonCharacter.BP_ThirdPersonCharacter_C|SetHoldSpawner _player true)
    (Audio|PlaySoundatLocation "/Game/Audio/coin-recieved.coin-recieved" (.location (Transformation|GetActorTransform _player)) "0, 0, 0" 1.0 1.0 0.0 0 0 0 0)
    (Actor|DestroyActor)))

(event EventBeginPlay
  ;[0.15 0.01297 0.1478 0.5] Reference Player
  (bind _asbp_third_person_character (Utilities|Casting|CastToBP_ThirdPersonCharacter (Game|Player|GetPlayerPawn 0)))
  (Variables|Default|SetPlayer _asbp_third_person_character))

(event Collision|EventActorBeginOverlap
  (params (OtherActor :type Actor%20Object%20Reference)))

(event EventTick
  (params (DeltaSeconds :type Float%20%28single-precision%29)))

(fn ConstructionScript)
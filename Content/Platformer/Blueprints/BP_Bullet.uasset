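; BP_Bullet is a projectile that damages the player's third-person character on contact.
; Each Tick moves it along a normalized local Direction by Speed, unswept and not scaled by delta time, then a Delay destroys it after LifeTime.
; The player pawn is cached on BeginPlay, and a mesh overlap with it calls DamagePlayer, then destroys the bullet after a short delay.
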(event OnComponentBeginOverlap(SM_Bullet)
  (params (OverlappedComponent :type Primitive%20Component%20Object%20Reference) (OtherActor :type Actor%20Object%20Reference) (OtherComp :type Primitive%20Component%20Object%20Reference) (OtherBodyIndex :type Integer) (bFromSweep :type Boolean) (SweepResult :type Hit%20Result%20Structure%20%28by%20ref%29))
  (bind _playerref (Variables|Default|GetPlayerRef))
  ;[0.15 0.15 0.15 0.5] Damage Player and Destroy self on contact with player
  (if (== OtherActor _playerref)
    (Default|DamagePlayer _playerref (Variables|Default|GetDamage))
    (Utilities|FlowControl|Delay 0.2)
    (Actor|DestroyActor)))

(event EventBeginPlay
  ;[0.15 0.15 0.15 0.5] Reference Player
  (bind _asbp_third_person_character (Utilities|Casting|CastToBP_ThirdPersonCharacter (Game|Player|GetPlayerPawn 0)))
  (Variables|Default|SetPlayerRef _asbp_third_person_character))

(event EventTick
  (params (DeltaSeconds :type Float%20%28single-precision%29))
  ;[0.15 0.15 0.15 0.5] Bullet Movement
  (Transformation|AddActorLocalOffset (* (Math|Vector|Normalize (Variables|Default|GetDirection)) (Variables|Default|GetSpeed)) false false)
  ;[0.15 0.15 0.15 0.5] Destroy Bullet after lifetime
  (Utilities|FlowControl|Delay (Variables|Default|GetLifeTime))
  (Actor|DestroyActor))

(fn ConstructionScript)